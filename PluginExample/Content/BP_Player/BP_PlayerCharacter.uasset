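; Player character Blueprint that connects pause input and hit feedback to the multiplayer player controller's UI.
; The pause input has player controller 0 create the pause menu widget, show the cursor and switch input away from the game.
; ShowHitMarkerBP casts the owning controller, takes its HUD widget and triggers the hit marker there.
; The construction script only calls its parent.
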(event Input|EnhancedActionEvents|EnhancedInputActionIA_Pause
  (params (ActionValue :type Boolean) (ElapsedSeconds :type Float%20%28double-precision%29) (TriggeredSeconds :type Float%20%28double-precision%29) (InputAction :type Input%20Action%20Object%20Reference :default "/Game/BP_Player/Input/IA_Pause.IA_Pause"))
  (:Started
    (bind _asbp_multiplayer_player_controller (Utilities|Casting|CastToBP_MultiplayerPlayerController (Game|GetPlayerController 0)))
    (Class|MultiplayerPlayerController|CreateUIWidget _asbp_multiplayer_player_controller "/Game/UI/BP_UI_PauseMenu.BP_UI_PauseMenu_C" 0 false 0 true true true false false false)))

(event EventShowHitMarkerBP
  (params (HitActor :type Actor%20Object%20Reference) (HitPhysicalMaterial :type Physical%20Material%20Object%20Reference))
  ;[0 0 0] Hit Marker
  (bind _asbp_multiplayer_player_controller (Utilities|Casting|CastToBP_MultiplayerPlayerController (Variables|Default|GetOwningController)))
  (bind _asbp_ui_player_hud (Utilities|Casting|CastToBP_UI_PlayerHUD (Variables|/Script/MultiplayerFPS.MultiplayerPlayerController|GetHUD _asbp_multiplayer_player_controller)))
  (Default|ShowHitMarker _asbp_ui_player_hud))

(fn ConstructionScript
  (|CallParentFunction))