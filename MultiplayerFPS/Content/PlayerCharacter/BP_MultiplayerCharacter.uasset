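; Multiplayer player character Blueprint implementing cosmetic and movement hooks for aiming, camera perspective and speed.
; Duration-scaled timelines play or reverse to blend aim FOV, arms transform and spring arm length for perspective and shoulder swaps.
; FOV changes go through a console command on the owning controller, and hit markers reach the HUD through the player controller.
; Speed requests pass through a server event to CurrentSpeed, whose OnRep sets max walk speed.
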(event Custom|Server%20Set%20Movement%20Speed%20BP
  (params (New%20Speed :type Float%20%28double-precision%29))
  ;[0 0 0] Movement
  (Variables|Default|SetCurrent%20Speed New%20Speed))

(event EventSetAimingFOVBP
  (params (Aiming :type Boolean) (AimingFOV :type Float%20%28single-precision%29) (TimeToAim :type Float%20%28single-precision%29))
  ;[0 0 0] Aiming
  (Components|Timeline|SetPlayRate (Variables|Default|GetAiming%20Set%20FOV%20Timeline) (/ 1.0 TimeToAim))
  (if Aiming
    (bind _new_fov (Timeline|Aiming%20Set%20FOV%20Timeline Play)
      (:Update
        (Class|MultiplayerCharacter|SetFOVBP (Math|Float|MapRangeClamped _new_fov 0.0 1.0 (Variables|Default|GetFieldOfView) AimingFOV)))
      (:Finished
        (Variables|Default|SetIsZoomingForAim false)))
    (else
      (Timeline|Aiming%20Set%20FOV%20Timeline Reverse))))

(event EventSetFOVBP
  (params (NewFOV :type Float%20%28single-precision%29))
  ;[0 0 0] FOV
  (Development|ExecuteConsoleCommand (Utilities|String|Append "FOV " (Utilities|String|ToString(Float) NewFOV)) (Variables|Default|GetOwningController))
  (Variables|Default|SetCurrentFOV NewFOV))

(event EventShowHitMarkerBP
  (params (HitActor :type Actor%20Object%20Reference) (HitPhysicalMaterial :type Physical%20Material%20Object%20Reference))
  ;[0 0 0] Hit Marker
  (bind _asbp_multiplayer_player_controller (Utilities|Casting|CastToBP_MultiplayerPlayerController (Variables|Default|GetOwningController)))
  (bind _asbp_ui_hud (Utilities|Casting|CastToBP_UI_HUD (Variables|/Script/MultiplayerFPS.MultiplayerPlayerController|GetHUD _asbp_multiplayer_player_controller)))
  (Default|ShowHitMarker _asbp_ui_hud))

(event EventSwitchPerspectiveBP
  (params (NewUsingThirdPerson :type Boolean) (SnapCameraLocation :type Boolean))
  ;[0 0 0] Perspective
  (|CallParentFunction NewUsingThirdPerson SnapCameraLocation)
  (if SnapCameraLocation
    (Variables|Default|SetIsSwitchingPerspective false :!label _label)
    (if (not NewUsingThirdPerson)
      (Class|MultiplayerCharacter|ApplyPerspectiveVisibility))
    (else
      (Components|Timeline|SetPlayRate (Variables|Default|GetSwitch%20Perspective%20Timeline) (/ 1.0 (Variables|Default|GetPerspectiveTransitionTime)))
      (if NewUsingThirdPerson
        (bind _value (Timeline|Switch%20Perspective%20Timeline Play)
          (:Update
            (bind _springarm (Variables|Default|GetSpringArm)
              (:then
                (Variables|/Script/Engine.SpringArmComponent|SetTargetArmLength _springarm (Math|Float|MapRangeClamped _value 0.0 1.0 (Variables|Default|GetFirstPersonSpringArmLength) (Class|MultiplayerCharacter|GetThirdPersonSpringArmLength))))
              (:else)))
          (:Finished
            (goto _label)))
        (else
          (Timeline|Switch%20Perspective%20Timeline Reverse))))))

(event EventSetThirdPersonShoulderBP
  (params (LeftShoulder :type Boolean) (SnapCameraLocation :type Boolean))
  ;[0 0 0] Perspective
  (|CallParentFunction LeftShoulder SnapCameraLocation)
  (if (and (Class|MultiplayerCharacter|GetUsingThirdPerson) (not SnapCameraLocation))
    (bind _current_length (CallFunction|StoreCurrentSpringArmLength))
    (Components|Timeline|SetPlayRate (Variables|Default|GetShoulder%20Swap%20Timeline) (/ 1.0 (Variables|Default|GetShoulderSwapTime)))
    (if LeftShoulder
      (bind _value (Timeline|Shoulder%20Swap%20Timeline Play)
        (:Update
          (bind _springarm (Variables|Default|GetSpringArm)
            (:then
              (Variables|/Script/Engine.SpringArmComponent|SetTargetArmLength _springarm (Math|Float|MapRangeClamped _value 0.0 1.0 _current_length (Class|MultiplayerCharacter|GetThirdPersonSpringArmLength))))
            (:else))))
      (else
        (Timeline|Shoulder%20Swap%20Timeline Reverse)))))

(event EventSetAimingArmsPositionBP
  (params (ArmsNormalLocation :type Vector :default "0, 0, 0") (ArmsNormalRotation :type Rotator :default "0, 0, 0") (ArmsAimLocation :type Vector :default "0, 0, 0") (ArmsAimRotation :type Rotator :default "0, 0, 0") (Aiming :type Boolean) (TimeToAim :type Float%20%28single-precision%29))
  (bind (_x _y _z) (Math|Vector|BreakVector ArmsAimLocation))
  (bind (_x_2 _y_2 _z_2) (Math|Vector|BreakVector ArmsNormalLocation))
  (bind (_roll _pitch _yaw) (Math|Rotator|BreakRotator ArmsNormalRotation))
  (bind (_roll_2 _pitch_2 _yaw_2) (Math|Rotator|BreakRotator ArmsAimRotation))
  ;[0 0 0] Aiming
  (Components|Timeline|SetPlayRate (Variables|Default|GetSet%20Aiming%20Arms%20Position%20Timeline) (/ 1.0 TimeToAim))
  (if Aiming
    (bind _value (Timeline|Set%20Aiming%20Arms%20Position%20Timeline Play)
      (:Update
        (bind _armsmesh (Variables|Default|GetArmsMesh)
          (:then
            (Transformation|SetRelativeLocationAndRotation _armsmesh (Math|Vector|MakeVector (Math|Float|MapRangeClamped _value 0.0 1.0 _x_2 _x) (Math|Float|MapRangeClamped _value 0.0 1.0 _y_2 _y) (Math|Float|MapRangeClamped _value 0.0 1.0 _z_2 _z)) (Math|Rotator|MakeRotator (Math|Float|MapRangeClamped _value 0.0 1.0 _roll _roll_2) (Math|Float|MapRangeClamped _value 0.0 1.0 _pitch _pitch_2) (Math|Float|MapRangeClamped _value 0.0 1.0 _yaw _yaw_2)) false false))
          (:else))))
    (else
      (Timeline|Set%20Aiming%20Arms%20Position%20Timeline Reverse))))

(event EventSetMovementSpeedBasedonSettingsBP
  (params (NewSpeed :type Float%20%28single-precision%29))
  ;[0 0 0] Movement
  (CallFunction|ServerSetMovementSpeedBP NewSpeed))

(fn ConstructionScript)

(fn StoreCurrentSpringArmLength
  (bind _springarm (Variables|Default|GetSpringArm)
    (:then
      (return (Variables|/Script/Engine.SpringArmComponent|GetTargetArmLength _springarm)))
    (:else)))

(fn OnRepCurrentSpeed
  (bind _charactermovement (Variables|Character|GetCharacterMovement)
    (:then
      (Variables|/Script/Engine.CharacterMovementComponent|SetMaxWalkSpeed _charactermovement (Variables|Default|GetCurrent%20Speed)))
    (:else
      (Development|PrintString "Character Movement Invalid BP_MultiplayerCharacter:OnRep_Current Speed" true true "(R=1.000000,G=0.000000,B=0.000000,A=1.000000)" 15.0))))