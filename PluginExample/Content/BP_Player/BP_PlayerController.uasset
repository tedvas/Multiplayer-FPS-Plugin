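; Player controller Blueprint that provides a runtime toggle between full and lowered graphics quality on the 5 key.
; Each press flips the LoweredGraphics flag and runs console commands for ray tracing, dynamic global illumination and reflection method.
; The lowered mode forces ray tracing effects off, disables dynamic GI and switches reflections from Lumen to screen space.
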(event Input|KeyboardEvents|5
  (params (Key :type Key%20Structure :default "None"))
  (bind _self self)
  (:Pressed
    (if (Variables|Default|GetLowered%20Graphics)
      (Variables|Default|SetLowered%20Graphics false)
      (Development|ExecuteConsoleCommand "r.RayTracing.ForceAllRayTracingEffects -1" _self)
      (Development|ExecuteConsoleCommand "r.DynamicGlobalilluminationMethod 1" _self)
      (Development|ExecuteConsoleCommand "r.ReflectionMethod 1" _self)
      (else
        (Variables|Default|SetLowered%20Graphics true)
        (Development|ExecuteConsoleCommand "r.RayTracing.ForceAllRayTracingEffects 0" _self)
        (Development|ExecuteConsoleCommand "r.DynamicGlobalilluminationMethod 0" _self)
        (Development|ExecuteConsoleCommand "r.ReflectionMethod 2" _self)))))

(fn ConstructionScript
  (|CallParentFunction))