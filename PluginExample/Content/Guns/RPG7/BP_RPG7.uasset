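; RPG-7 weapon Blueprint that hides the loaded rocket when fired and shows it again on reload.
; Fire and client-fire events set the HideRocket flag, while reload and server-reload events clear it.
; Its RepNotify applies the flag to both the Rocket and ThirdPersonRocket components, skipping the visibility change when InfiniteAmmo equals 2.
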(event EventFireBP
  (Variables|Default|SetHide%20Rocket true))

(event EventReloadBP
  (Variables|Default|SetHide%20Rocket false))

(event EventClientFireBP
  (Variables|Default|SetHide%20Rocket true))

(event EventServerReloadBP
  (Variables|Default|SetHide%20Rocket false))

(fn ConstructionScript
  (|CallParentFunction))

(fn OnRepHideRocket
  (if (!= (Variables|Default|GetInfiniteAmmo) 2)
    (Development|SetHiddeninGame (Variables|Default|GetRocket) (Variables|Default|GetHide%20Rocket) false)))