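; Master multiplayer gun Blueprint that handles recoil, charge-up, overheating and continuous-fire effects.
; Timelines drive control-rotation recoil, charge progress and heat, reversing for cancel and cooldown.
; Heat can toggle muzzle smoke and flags overheat, and a finished cooldown can resume held fire.
; Muzzle flash, looping fire sound and smoke pass through Server-then-Multicast events, with validity checks preventing duplicate attached components.
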(event Custom|Client%20Add%20Recoil
  (bind _returnvalue (Class|MultiplayerGun|GetOwningPlayer))
  (bind _returnvalue_2 (Pawn|GetController _returnvalue))
  (bind _returnvalue_3 (Pawn|GetControlRotation _returnvalue_2 :!class /Script/Engine.Controller))
  ;[0 0 0] Recoil
  (bind _value (Timeline|Recoil%20Interpolation PlayFromStart)
    (:Update
      (Utilities|IsValid _returnvalue
        (:Is%20Valid
          (Utilities|IsValid _returnvalue_2
            (:Is%20Valid
              (Pawn|SetControlRotation _returnvalue_2 (Math|Rotator|MakeRotator (.roll _returnvalue_3) (Math|Float|MapRangeClamped _value 0.0 1.0 (.pitch _returnvalue_3) (+ (.pitch _returnvalue_3) (Variables|Default|GetVerticalRecoil))) (Math|Float|MapRangeClamped _value 0.0 1.0 (.yaw _returnvalue_3) (+ (.yaw _returnvalue_3) (Variables|Default|GetHorizontalRecoil))))))))))))

(event Custom|Server%20Continuous%20Fire%20BP
  ;[0 0 0] Continuous Fire
  (CallFunction|MulticastContinuousFireBP))

(event Custom|Multicast%20Continuous%20Fire%20BP
  (bind _returnvalue (Class|MultiplayerGun|GetFireScenetoUse))
  ;[0 0 0] Continuous Fire
  (Utilities|IsValid (Variables|Default|GetSpawnedContinuousMuzzleFlash)
    (:Is%20Valid
      _)
    (:Is%20Not%20Valid
      (bind _returnvalue_2 (Effects|SpawnEmitterAttached (Variables|Default|GetMuzzleFlash) _returnvalue "None"))
      (Variables|Default|SetSpawnedContinuousMuzzleFlash _returnvalue_2)))
  (Utilities|IsValid (Variables|Default|GetSpawnedContinuousFireSound)
    (:Is%20Not%20Valid
      (bind _returnvalue_3 (Audio|SpawnSoundAttached (Variables|Default|GetFireSound) _returnvalue "None" "0, 0, 0" "0, 0, 0" "KeepRelativeOffset" true 1.0 1.0 0.0 0 0))
      (Variables|Default|SetSpawnedContinuousFireSound _returnvalue_3))))

(event Custom|Server%20Stop%20Continuous%20Fire%20BP
  ;[0 0 0] Continuous Fire
  (CallFunction|MulticastStopContinuousFireBP))

(event Custom|Multicast%20Stop%20Continuous%20Fire%20BP
  ;[0 0 0] Continuous Fire
  (Utilities|IsValid (Variables|Default|GetSpawnedContinuousFireSound)
    (:Is%20Valid
      (Audio|Components|Audio|SetVolumeMultiplier (Variables|Default|GetSpawnedContinuousFireSound) 0.0 :!class /Script/Engine.AudioComponent)
      (Components|DestroyComponent (Variables|Default|GetSpawnedContinuousFireSound))
      (Variables|Default|SetSpawnedContinuousFireSound 0))
    (:Is%20Not%20Valid
      _))
  (Utilities|IsValid (Variables|Default|GetSpawnedContinuousMuzzleFlash)
    (:Is%20Valid
      (Components|DestroyComponent (Variables|Default|GetSpawnedContinuousMuzzleFlash))
      (Variables|Default|SetSpawnedContinuousMuzzleFlash 0))))

(event Custom|Server%20Spawn%20Smoke%20Effect%20BP
  ;[0 0 0] Smoke Effect
  (CallFunction|MulticastSpawnSmokeEffectBP))

(event Custom|Multicast%20Spawn%20Smoke%20Effect%20BP
  (bind _returnvalue (Class|MultiplayerGun|GetFireScenetoUse))
  ;[0 0 0] Smoke Effect
  (Utilities|IsValid (Variables|Default|GetSpawnedSmokeEffect)
    (:Is%20Valid
      _)
    (:Is%20Not%20Valid
      (bind _returnvalue_2 (Effects|SpawnEmitterAttached (Variables|Default|GetSmokeEffectToSpawn) _returnvalue "None"))
      (Variables|Default|SetSpawnedSmokeEffect _returnvalue_2)))
  (Utilities|IsValid (Variables|Default|GetSpawnedSmokeSound)
    (:Is%20Not%20Valid
      (bind _returnvalue_3 (Audio|SpawnSoundAttached (Variables|Default|GetSmokeSoundToSpawn) _returnvalue "None" "0, 0, 0" "0, 0, 0" "KeepRelativeOffset" true 1.0 1.0 0.0 0 0))
      (Variables|Default|SetSpawnedSmokeSound _returnvalue_3))))

(event Custom|Server%20Destroy%20Smoke%20Effect%20BP
  ;[0 0 0] Smoke Effect
  (CallFunction|MulticastDestroySmokeEffectBP))

(event Custom|Multicast%20Destroy%20Smoke%20Effect%20BP
  ;[0 0 0] Smoke Effect
  (if (and (Utilities|IsValid (Variables|Default|GetSpawnedSmokeEffect)) (Variables|Default|GetDestroySmokeEffectWhenNotShooting))
    (Components|DestroyComponent (Variables|Default|GetSpawnedSmokeEffect))
    (Variables|Default|SetSpawnedSmokeEffect 0))
  (if (and (Utilities|IsValid (Variables|Default|GetSpawnedSmokeSound)) (Variables|Default|GetDestroySmokeSoundWhenNotShooting))
    (Audio|Components|Audio|SetVolumeMultiplier (Variables|Default|GetSpawnedSmokeSound) 0.0 :!class /Script/Engine.AudioComponent)
    (Components|DestroyComponent (Variables|Default|GetSpawnedSmokeSound))
    (Variables|Default|SetSpawnedSmokeSound 0)))

(event EventAddRecoilBP
  ;[0 0 0] Recoil
  (CallFunction|ClientAddRecoil))

(event EventContinuousFireBP
  ;[0 0 0] Continuous Fire
  (CallFunction|ServerContinuousFireBP))

(event EventCancelChargeUpBP
  (bind _returnvalue (Class|MultiplayerGun|GetChargeUpTime))
  ;[0 0 0] Charge Up
  (Components|Timeline|SetPlayRate (Variables|Default|GetCharge%20Timeline) (/ 1.0 _returnvalue))
  (bind _value (Timeline|Charge%20Timeline Reverse)
    (:Update
      (Variables|Default|SetCurrentChargeUpProgress (Math|Float|MapRangeClamped _value 0.0 1.0 0.0 _returnvalue)))))

(event EventSetChargeUpProgressTimeforTimeline
  (params (NewTime :type Float%20%28single-precision%29))
  ;[0 0 0] Charge Up
  (bind _value (Timeline|Charge%20Timeline SetNewTime)
    (:Update
      (Variables|Default|SetCurrentChargeUpProgress (Math|Float|MapRangeClamped _value 0.0 1.0 0.0 (Class|MultiplayerGun|GetChargeUpTime))))))

(event EventCoolDownBP
  (bind _returnvalue (Class|MultiplayerGun|GetOwningPlayerCast))
  (bind _maxheat (Variables|Default|GetMaxHeat))
  ;[0 0 0] Overheating
  (Components|Timeline|SetPlayRate (Variables|Default|GetContinuous%20Fire%20Overheat) (/ 1.0 (Variables|Default|GetTimeToCooldown)))
  (bind _overheat_value (Timeline|Continuous%20Fire%20Overheat Reverse)
    (:Update
      (Variables|Default|SetCurrentHeat (Math|Float|MapRangeClamped _overheat_value 0.0 1.0 0.0 _maxheat))
      (if (== (Variables|Default|GetSpawnSmokeEffectWhenShooting) 2)
        (if (>= (/ (Math|Float|MapRangeClamped _overheat_value 0.0 1.0 0.0 _maxheat) (Variables|Default|GetMaxHeat)) (Variables|Default|GetPercentageOfOverheatToSpawnSmoke))
          (Class|MultiplayerGun|SpawnSmokeEffectBP)
          (else
            (Class|MultiplayerGun|DestroySmokeEffectBP)))))
    (:Finished
      (if (>= (Variables|Default|GetCurrentHeat) _maxheat)
        (Variables|Default|SetReachedMaxHeat true)
        (else
          (Variables|Default|SetReachedMaxHeat false)
          (if (!= (Variables|Default|GetFireMode) 0)
            (if (Variables|/Script/MultiplayerFPS.MultiplayerCharacter|GetHoldingFireInput _returnvalue)
              (Class|MultiplayerCharacter|Fire _returnvalue))))))))

(event EventPrintDistanceTravedBP
  (params (Distance :type Float%20%28single-precision%29))
  ;[0 0 0] Debugging
  (Development|PrintString (Utilities|String|ToString(Float) Distance)))

(event EventDestroyed
  (bind _spawnedcontinuousfiresound (Variables|Default|GetSpawnedContinuousFireSound))
  ;[0 0 0] Destroyed
  (|CallParentFunction)
  (Utilities|IsValid _spawnedcontinuousfiresound
    (:Is%20Valid
      (Components|DestroyComponent _spawnedcontinuousfiresound))))

(event EventStopContinuousFireBP
  ;[0 0 0] Continuous Fire
  (CallFunction|ServerStopContinuousFireBP))

(event EventDestroySmokeEffectBP
  ;[0 0 0] Smoke Effect
  (CallFunction|ServerDestroySmokeEffectBP))

(event EventSpawnSmokeEffectBP
  ;[0 0 0] Smoke Effect
  (CallFunction|ServerSpawnSmokeEffectBP))

(event EventOverheatBP
  (bind _returnvalue (Class|MultiplayerGun|GetOwningPlayerCast))
  (bind _maxheat (Variables|Default|GetMaxHeat))
  ;[0 0 0] Overheating
  (Components|Timeline|SetPlayRate (Variables|Default|GetContinuous%20Fire%20Overheat) (/ 1.0 (Variables|Default|GetTimeToOverheat)))
  (bind _overheat_value (Timeline|Continuous%20Fire%20Overheat Play)
    (:Update
      (Variables|Default|SetCurrentHeat (Math|Float|MapRangeClamped _overheat_value 0.0 1.0 0.0 _maxheat))
      (if (== (Variables|Default|GetSpawnSmokeEffectWhenShooting) 2)
        (if (>= (/ (Math|Float|MapRangeClamped _overheat_value 0.0 1.0 0.0 _maxheat) (Variables|Default|GetMaxHeat)) (Variables|Default|GetPercentageOfOverheatToSpawnSmoke))
          (Class|MultiplayerGun|SpawnSmokeEffectBP)
          (else
            (Class|MultiplayerGun|DestroySmokeEffectBP)))))
    (:Finished
      (if (>= (Variables|Default|GetCurrentHeat) _maxheat)
        (Variables|Default|SetReachedMaxHeat true)
        (else
          (Variables|Default|SetReachedMaxHeat false)
          (if (!= (Variables|Default|GetFireMode) 0)
            (if (Variables|/Script/MultiplayerFPS.MultiplayerCharacter|GetHoldingFireInput _returnvalue)
              (Class|MultiplayerCharacter|Fire _returnvalue))))))))

(event EventChargeUpBP
  (bind _returnvalue (Class|MultiplayerGun|GetChargeUpTime))
  ;[0 0 0] Charge Up
  (Components|Timeline|SetPlayRate (Variables|Default|GetCharge%20Timeline) (/ 1.0 _returnvalue))
  (bind _value (Timeline|Charge%20Timeline Play)
    (:Update
      (Variables|Default|SetCurrentChargeUpProgress (Math|Float|MapRangeClamped _value 0.0 1.0 0.0 _returnvalue)))))

(fn ConstructionScript)